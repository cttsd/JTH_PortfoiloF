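; Slime monster 03 Blueprint whose graph keeps the monster's health bar widget up to date.
; Each Tick it casts the Widget component's content to WBP_HPBar and sets the HP element's horizontal render scale to HP / MAXHP.
; BeginPlay, overlap and construction are empty, and an unconnected branch repeats the bar update or sets the widget background transparent.
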(event EventBeginPlay)

(event Collision|EventActorBeginOverlap
  (params (OtherActor :type Actor%20Object%20Reference)))

(event EventTick
  (params (DeltaSeconds :type Float%20%28single-precision%29))
  (bind _aswbp_hpbar (Utilities|Casting|CastToWBP_HPBar (UserInterface|GetWidget (Variables|Default|GetWidget))))
  (Widget|Transform|SetRenderScale (Variables|/Game/BluePrint/GamePlayeBluePrint/GameUI/WBP_HPBar.WBP_HPBar_C|GetHP _aswbp_hpbar) (Math|Vector2D|MakeVector2D (/ (Variables|Default|GetHP) (Variables|Default|GetMAXHP)) 1.0)))

(fn ConstructionScript)